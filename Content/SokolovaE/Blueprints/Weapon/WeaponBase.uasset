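; WeaponBase is a weapon actor that automatically fires once per second from BeginPlay through a looping delay.
; Each shot checks and spends one round via the AmmoACC component, then spawns an AmmoBase projectile at the Arrow's transform.
; When out of ammo it plays a snap sound instead, and every attempt updates the Ammo text to show current and maximum rounds.
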(event Custom|Fire
  (bind _ammoacc (Variables|Default|GetAmmoACC))
  (Utilities|FlowControl|Sequence
    (:then_0
      (if (Default|CheckAmmo _ammoacc 1)
        (Default|SubstractAmmo _ammoacc 1)
        (Game|SpawnActorfromClass "/Game/SokolovaE/Blueprints/Weapon/AmmoBase.AmmoBase_C" (Transformation|GetWorldTransform (Variables|Default|GetArrow)) "AlwaysSpawn" 0 0)
        (else
          (Audio|SpawnSoundatLocation "/Engine/VREditor/Sounds/UI/Object_Snaps_To_Another_Actor.Object_Snaps_To_Another_Actor" (Transformation|GetActorLocation) "0, 0, 0" 1.0 1.0 0.0 0 0))))
    (:then_1
      (Rendering|Components|TextRender|SetText (Variables|Default|GetAmmo) (Utilities|Text|FormatText "{current}/{max}" (Variables|/Game/SokolovaE/Blueprints/Weapon/AmmoACC.AmmoACC_C|GetCurrentAmmo (Variables|Default|GetAmmoACC)) (Variables|/Game/SokolovaE/Blueprints/Weapon/AmmoACC.AmmoACC_C|GetMaxAmmo (Variables|Default|GetAmmoACC)))))))

(event EventBeginPlay
  (Utilities|FlowControl|Delay 1.0 :!label _label)
  (CallFunction|Fire)
  (goto _label))

(fn ConstructionScript)