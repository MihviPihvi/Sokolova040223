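; AmmoACC is a weapon ammo component that tracks a current round count against a maximum.
; It fills the count to the maximum on BeginPlay.
; SubstractAmmo lowers the count by a given amount, clamped between zero and the maximum, and CheckAmmo reports whether enough remains to cover a requested amount.
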(event EventBeginPlay
  (Variables|Default|SetCurrentAmmo (Variables|Default|GetMaxAmmo)))

(event EventTick
  (params (DeltaSeconds :type Float%20%28single-precision%29)))

(fn SubstractAmmo
  (params (Value :type Integer))
  (Variables|Default|SetCurrentAmmo (Math|Integer|Clamp(Integer) (- (Variables|Default|GetCurrentAmmo) Value) 0 (Variables|Default|GetMaxAmmo))))

(fn CheckAmmo
  (params (Value :type Integer))
  (return (>= (Variables|Default|GetCurrentAmmo) Value)))