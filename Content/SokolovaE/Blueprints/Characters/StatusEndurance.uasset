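; StatusEndurance is a Blueprint that holds a character's endurance value, filled to MaxEndurance on BeginPlay.
; ReduceEndurance sets CurrentEndurance to MaxEndurance minus the given value, clamped between zero and the maximum, so successive reductions do not accumulate.
; Tick does nothing, and a debug print of the current value is left disconnected.
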(event EventTick
  (params (DeltaSeconds :type Float%20%28single-precision%29)))

(event EventBeginPlay
  (Variables|Default|SetCurrentEndurance (Variables|Default|GetMaxEndurance)))

(fn ReduceEndurance
  (params (Value :type Float%20%28single-precision%29))
  (if true
    (Variables|Default|SetCurrentEndurance (Math|Float|Clamp(Float) (- (Variables|Default|GetMaxEndurance) Value) 0.0 (Variables|Default|GetMaxEndurance)))))