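; StatusAC, by its name an actor component for character status, tracks current health against a maximum.
; It fills health to the maximum on BeginPlay and prints the current value on screen every tick.
; MakeDamageHealth heals or damages by a fixed one point according to a boolean, clamped between zero and the maximum; its Value input is unused.
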(event EventTick
  (params (DeltaSeconds :type Float%20%28single-precision%29))
  (Development|PrintString (Utilities|String|ToString(Float) (Variables|Default|GetCurrentHP)) true true "(R=0.000000,G=0.660000,B=1.000000,A=1.000000)" DeltaSeconds))

(event EventBeginPlay
  (Variables|Default|SetCurrentHP (Variables|Default|GetMaxHP))
  (Utilities|FlowControl|Delay 1.0))

(fn MakeDamage/Health
  (params (Value :type Float%20%28single-precision%29) (IsHeal :type Boolean))
  (if IsHeal
    (Variables|Default|SetCurrentHP (Math|Float|Clamp(Float) (+ (Variables|Default|GetCurrentHP) 1.0) 0.0 (Variables|Default|GetMaxHP)))
    (else
      (Variables|Default|SetCurrentHP (Math|Float|Clamp(Float) (- (Variables|Default|GetCurrentHP) 1.0) 0.0 (Variables|Default|GetMaxHP))))))