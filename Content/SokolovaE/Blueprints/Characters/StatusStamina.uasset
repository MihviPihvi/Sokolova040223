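; StatusStamina tracks a stamina value for characters, starting at MaxStamina on BeginPlay.
; StaminaLossGain subtracts the passed value and clamps the result between zero and the maximum, so negative values restore stamina.
; Tick prints the current stamina to screen every frame as a debug readout.
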(event EventTick
  (params (DeltaSeconds :type Float%20%28single-precision%29))
  (Development|PrintString (Utilities|String|ToString(Float) (Variables|Default|GetCurrentStamina)) true true "(R=1.000000,G=0.163742,B=0.713442,A=1.000000)" DeltaSeconds))

(event EventBeginPlay
  (Variables|Default|SetCurrentStamina (Variables|Default|GetMaxStamina)))

(fn StaminaLoss/Gain
  (params (Value :type Float%20%28single-precision%29))
  (if true
    (Variables|Default|SetCurrentStamina (Math|Float|Clamp(Float) (- (Variables|Default|GetCurrentStamina) Value) 0.0 (Variables|Default|GetMaxStamina)))))