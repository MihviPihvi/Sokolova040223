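; BP_Female_Character is a character Blueprint that handles jump and sprint input.
; The Jump action sets the jump Z velocity on CharacterMovement just before jumping, and stops jumping on release.
; The Sprint action raises max walk speed while held and sets it back to a fixed walking value on release.
; The construction script only calls its parent.
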(event Input|ActionEvents|InputActionSprint
  (params (Key :type Key%20Structure :default "None"))
  (:Pressed
    (Variables|/Script/Engine.CharacterMovementComponent|SetMaxWalkSpeed (Variables|Character|GetCharacterMovement) 1.2e+03))
  (:Released
    (Variables|/Script/Engine.CharacterMovementComponent|SetMaxWalkSpeed (Variables|Character|GetCharacterMovement) 5e+02)))

(event Input|ActionEvents|InputActionJump
  (params (Key :type Key%20Structure :default "None"))
  ;[1 1 1] Прыжок
  (:Pressed
    (Variables|/Script/Engine.CharacterMovementComponent|SetJumpZVelocity (Variables|Character|GetCharacterMovement) 9e+02)
    (Character|Jump))
  (:Released
    (Character|StopJumping)))

(fn ConstructionScript
  (|CallParentFunction))