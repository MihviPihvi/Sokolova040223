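; BP_Male_CharacterSyna is a male character Blueprint that adds jump and sprint input handling.
; Jump input sets the jump Z velocity on each press before jumping, and stops the jump on release.
; Sprint input raises the CharacterMovement max walk speed while held and drops it to a fixed walking speed on release.
; The construction script only calls its parent.
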(event Input|ActionEvents|InputActionSprint
  (params (Key :type Key%20Structure))
  (:Pressed
    (Variables|/Script/Engine.CharacterMovementComponent|SetMaxWalkSpeed (Variables|Character|GetCharacterMovement) 6e+02))
  (:Released
    (Variables|/Script/Engine.CharacterMovementComponent|SetMaxWalkSpeed (Variables|Character|GetCharacterMovement) 4e+02)))

(event Input|ActionEvents|InputActionJump
  (params (Key :type Key%20Structure))
  (:Pressed
    (Variables|/Script/Engine.CharacterMovementComponent|SetJumpZVelocity (Variables|Character|GetCharacterMovement) 2.5e+02)
    (Character|Jump))
  (:Released
    (Character|StopJumping)))

(fn ConstructionScript
  (|CallParentFunction))