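; Door_2 is an interactable door Blueprint that swings open and closed around its yaw axis.
; The interact interface event alternates through a FlipFlop between playing and reversing a timeline, which drives the door's relative rotation up to a quarter turn.
; A separate overlap component shows the open-door button widget when BP_MainCharacter enters and removes it on exit.
; The OpenDoor event is an empty stub.
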(event OnComponentBeginOverlap(Door_ButtonSW)
  (params (OverlappedComponent :type Primitive%20Component%20Object%20Reference) (OtherActor :type Actor%20Object%20Reference) (OtherComp :type Primitive%20Component%20Object%20Reference) (OtherBodyIndex :type Integer) (bFromSweep :type Boolean) (SweepResult :type Hit%20Result%20Structure%20%28by%20ref%29))
  (Utilities|Casting|CastToBP_MainCharacter OtherActor)
  (bind _returnvalue (UserInterface|CreateWidget "/Game/SokolovaE/Blueprints/GUI/Button_Open_Door.Button_Open_Door_C"))
  (UserInterface|Viewport|AddtoViewport _returnvalue 0))

(event OnComponentEndOverlap(Door_ButtonSW)
  (params (OverlappedComponent :type Primitive%20Component%20Object%20Reference) (OtherActor :type Actor%20Object%20Reference) (OtherComp :type Primitive%20Component%20Object%20Reference) (OtherBodyIndex :type Integer))
  (Utilities|Casting|CastToBP_MainCharacter OtherActor)
  (Widget|RemovefromParent (stale OnComponentBeginOverlap(Door_ButtonSW) _returnvalue)))

(event Custom|OpenDoor)

(event EventInteractInterfaceFC
  (Utilities|FlowControl|FlipFlop
    (:A
      (bind _beta (Timeline|OpenDoorTL Play)
        (:Update
          (Transformation|SetRelativeRotation (Variables|Default|GetDoor) (Math|Rotator|MakeRotator 0.0 0.0 (* _beta -9e+01)) false false))))
    (:B
      (Timeline|OpenDoorTL Reverse))))

(fn ConstructionScript)